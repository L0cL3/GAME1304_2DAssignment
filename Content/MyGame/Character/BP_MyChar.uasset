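; Side-scrolling 2D player character with Mario flipbook animations, able to walk left and right and jump.
; MoveRight input moves it along world X and rotates the sprite 180 degrees to face the direction of travel.
; Jump input switches to the jump flipbook, while Tick picks walk or idle from velocity whenever it is not falling.
; Landing resets the sprite to idle.
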(event `InputAxis|MoveRight`
  (params (AxisValue :type "Float (single-precision)"))
  (bind _sprite (`self.Sprite`))
  (if (> AxisValue 0.0)
    (set `self.isMovingRight` true)
    (`self.AddMovementInput` (1.0 0.0 0.0) AxisValue :!label _label)
    (if (`self.isMovingRight`)
      (`SceneComponent.K2_SetRelativeRotation` :`self` _sprite)
      (else
        (`SceneComponent.K2_SetRelativeRotation` _sprite (struct :`Yaw` 180.0) false false)))
    (elif (< AxisValue 0.0)
      (set `self.isMovingRight` false)
      (goto _label))))

(event `InputAction|Jump`
  (params (Key :type "Key Structure"))
  (:`Pressed`
    (`self.Jump`)
    (`PaperFlipbookComponent.SetFlipbook` (`self.Sprite`) "/Game/MyGame/Character/Flipbook/FB_mario_jump.FB_mario_jump"))
  (:`Released`
    (`self.StopJumping`)))

(event `self.ReceiveTick`
  (params (DeltaSeconds :type "Float (single-precision)"))
  (if (not (`NavMovementComponent.IsFalling` (`self.CharacterMovement`)))
    (`PaperFlipbookComponent.SetFlipbook` (`self.Sprite`) (select `bool` (> (`KismetMathLibrary.VSize` (`self.GetVelocity`)) 0.0) :`false` "/Game/MyGame/Character/Flipbook/FB_mario_idle.FB_mario_idle" :`true` "/Game/MyGame/Character/Flipbook/FB_mario_walk.FB_mario_walk" :!type "PaperFlipbook Object Reference"))))

(event `self.OnLanded`
  (params (Hit :type "HitResult Structure (by ref)"))
  (`PaperFlipbookComponent.SetFlipbook` (`self.Sprite`) "/Game/MyGame/Character/Flipbook/FB_mario_idle.FB_mario_idle"))

(fn `UserConstructionScript`)