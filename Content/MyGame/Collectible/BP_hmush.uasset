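; BP_hmush is a health pickup collectible that heals the player character on overlap.
; When a BP_MyChar overlaps it, it adds a fixed amount to that character's Health, capped at the maximum of 100.
; It then plays the item sound at its location and destroys itself through its render component's owner.
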(event `self.ReceiveActorBeginOverlap`
  (params (OtherActor :type "Actor Object Reference"))
  (bind _asbp_my_char (cast `/Game/MyGame/Character/BP_MyChar` OtherActor))
  (bind _returnvalue (+ (`/Game/MyGame/Character/BP_MyChar.health` _asbp_my_char) 30))
  (if (> _returnvalue 100)
    (set `/Game/MyGame/Character/BP_MyChar.health` 100 _asbp_my_char)
    (else
      (set `/Game/MyGame/Character/BP_MyChar.health` _returnvalue _asbp_my_char)))
  (`GameplayStatics.PlaySoundAtLocation` "/Game/MyGame/Sound/Cue/Item_Cue.Item_Cue" (`self.K2_GetActorLocation`) (struct) 1.0 1.0 0.0 null null null)
  (`self.K2_DestroyActor` (`ActorComponent.GetOwner` (`self.RenderComponent`))))

(fn `UserConstructionScript`)