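; BP_Cloud is an enemy-folder cloud actor that drifts back and forth horizontally between AI blocker actors.
; Each tick it shifts its RenderComponent along local X by a fixed step, with the sign chosen by the Ismovingright flag.
; Overlapping a BP_AIBlock flips that flag to reverse direction.
; Movement is unswept and not scaled by delta time, so speed depends on frame rate.
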(event `self.ReceiveActorBeginOverlap`
  (params (OtherActor :type "Actor Object Reference"))
  (cast `/Game/MyGame/Enemies/BP_AIBlock` OtherActor)
  (set `self.ismovingright` (not (`self.ismovingright`))))

(event `self.ReceiveTick`
  (params (DeltaSeconds :type "Float (single-precision)"))
  (`SceneComponent.K2_AddLocalTransform` (`self.RenderComponent`) (select `bool` (`self.ismovingright`) :`false` (`KismetMathLibrary.MakeTransform` (0.6 0.0 0.0)) :`true` (`KismetMathLibrary.MakeTransform` (-0.6 0.0 0.0))) false false))

(fn `UserConstructionScript`)