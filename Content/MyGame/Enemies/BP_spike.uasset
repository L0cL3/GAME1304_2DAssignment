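; BP_spike is a moving hazard that takes 10 Health from BP_MyChar on overlap, flags it as damaged and calls Play.
; Each Tick sets the render component's rotation from Ismovingright, flipping it 180 degrees, then nudges it along negative local X.
; The step grows while the character found by GetActorOfClass has IsDmged set, and is per frame, unscaled by delta time.
; Ismovingright and the reset of IsDmged are not handled here.
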(event `self.ReceiveActorBeginOverlap`
  (params (OtherActor :type "Actor Object Reference"))
  (bind _asbp_my_char (cast `/Game/MyGame/Character/BP_MyChar` OtherActor))
  (set `/Game/MyGame/Character/BP_MyChar.health` (+ (`/Game/MyGame/Character/BP_MyChar.health` _asbp_my_char) -10) _asbp_my_char)
  (set `/Game/MyGame/Character/BP_MyChar.isDmged` true _asbp_my_char)
  (`AudioComponent.Play` 0.0))

(event `self.ReceiveTick`
  (params (DeltaSeconds :type "Float (single-precision)"))
  (bind _rendercomponent (`self.RenderComponent`))
  (if (`self.ismovingright`)
    (`SceneComponent.K2_SetRelativeRotation` _rendercomponent (struct :`Yaw` 180.0) false false)
    (else
      (`SceneComponent.K2_SetRelativeRotation` _rendercomponent (struct) false false)))
  (bind _returnvalue (`GameplayStatics.GetActorOfClass` "/Game/MyGame/Character/BP_MyChar.BP_MyChar_C"))
  (`SceneComponent.K2_AddLocalTransform` (`self.RenderComponent`) (select `bool` (`/Game/MyGame/Character/BP_MyChar.isDmged` _returnvalue) :`false` (`KismetMathLibrary.MakeTransform` (-0.3 0.0 0.0)) :`true` (`KismetMathLibrary.MakeTransform` (-0.8 0.0 0.0))) false false))

(fn `UserConstructionScript`)